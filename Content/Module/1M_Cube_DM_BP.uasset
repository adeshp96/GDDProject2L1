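; Destructible moving cube actor that breaks apart with radial damage when hit by a FirstPersonProjectile.
; Overlapping its PresenceCheck enables input, letting StartMovingPlatform slide it along X via a timeline.
; It then spins and circles on Tick using sine/cosine offsets, while a second timeline drives its height.
; When that timeline ends, the cube applies radial damage to its Destructible and loads StarterMap after a short delay.
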(event `self.ReceiveHit`
  (params (MyComp :type "PrimitiveComponent Object Reference") (Other :type "Actor Object Reference") (OtherComp :type "PrimitiveComponent Object Reference") (bSelfMoved :type Boolean) (HitLocation :type "Vector Structure") (HitNormal :type "Vector Structure") (NormalImpulse :type "Vector Structure") (Hit :type "HitResult Structure (by ref)"))
  ;[1 1 1] Destroy when shot
  (cast `/Game/FirstPersonBP/Blueprints/FirstPersonProjectile` Other)
  (`DestructibleComponent.ApplyRadiusDamage` (`self.Destructible`) 5.0 HitLocation 100.0 10000.0 false))

(event `self.PresenceCheck.OnComponentBeginOverlap`
  (params (OverlappedComponent :type "PrimitiveComponent Object Reference") (OtherActor :type "Actor Object Reference") (OtherComp :type "PrimitiveComponent Object Reference") (OtherBodyIndex :type Integer) (bFromSweep :type Boolean) (SweepResult :type "HitResult Structure (by ref)"))
  ;[1 1 1] Start Capturing Input
  (`self.EnableInput` (`GameplayStatics.GetPlayerController` 0)))

(event `InputAction|StartMovingPlatform`
  (params (Key :type "Key Structure"))
  (bind (_returnvalue_x _returnvalue_y _returnvalue_z) (`KismetMathLibrary.BreakVector` (`self.K2_GetActorLocation`)))
  (bind _destructible (`self.Destructible`))
  (bind (_returnvalue_x_2 _returnvalue_y_2 _returnvalue_z_2) (`KismetMathLibrary.BreakVector` (`SceneComponent.K2_GetComponentLocation` _destructible)))
  ;[1 1 1] Move Platform Above Target
  (:`Pressed`
    (bind (_direction _platformx) (`Timeline|Timeline_0`)
      (:`Update`
        (`self.K2_SetActorLocation` (`KismetMathLibrary.MakeVector` _platformx _returnvalue_y _returnvalue_z)))
      (:`Finished`
        (set `self.StartCircularMotion?` true)
        ;[1 1 1] Perform Rotatory Motion
        (bind (_direction_2 _zvalue) (`Timeline|Timeline_1` :!via `PlayFromStart`)
          (:`Finished`
            (`DestructibleComponent.ApplyRadiusDamage` _destructible 5.0 (`KismetMathLibrary.MakeVector` _returnvalue_x_2 _returnvalue_y_2 _returnvalue_z_2) 100.0 10000.0 false)
            (`KismetSystemLibrary.Delay` 3.0)
            (`GameplayStatics.OpenLevel` "StarterMap")))))))

(event `self.ReceiveTick`
  (params (DeltaSeconds :type "Float (single-precision)"))
  (bind (_returnvalue_x _returnvalue_y) (`KismetMathLibrary.BreakVector` (`self.K2_GetActorLocation`)))
  (bind _returnvalue (`KismetSystemLibrary.GetGameTimeInSeconds`))
  ;[1 1 1] Perform Rotatory Motion
  (if (`self.StartCircularMotion?`)
    (`self.K2_AddActorLocalRotation` (`KismetMathLibrary.MakeRotator` 0.0 0.0 (`GameplayStatics.GetWorldDeltaSeconds`)))
    (`self.K2_SetActorLocation` (`KismetMathLibrary.MakeVector` (+ _returnvalue_x (* (`KismetMathLibrary.Sin` _returnvalue) 20.0)) (+ _returnvalue_y (* (`KismetMathLibrary.Cos` _returnvalue) 20.0)) (stale `InputAction|StartMovingPlatform` _zvalue)))))

(fn `UserConstructionScript`)